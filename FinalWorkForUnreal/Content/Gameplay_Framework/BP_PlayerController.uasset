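; BP_PlayerController is a player controller that turns axis input into movement and look control for the possessed BP_Character.
; On possession it stores the pawn and caches it as a BP_Character if the cast succeeds.
; Forward and Right axes add movement input along that character's forward and right vectors, while Turn and LookUp feed the controller's yaw and pitch.
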(event `self.ReceivePossess`
  (params (PossessedPawn :type "Pawn Object Reference"))
  (bind _output_get (set `self.Possessed Pawn` PossessedPawn))
  (bind _asbp_character (cast `/Game/Gameplay_Framework/BP_Character` _output_get))
  (set `self.BP Character` _asbp_character))

(event `InputAxis|Forward`
  (params (AxisValue :type "Float (single-precision)"))
  (bind _bp_character (`self.BP Character`))
  ;[1 1 1] Move
  (`Pawn.AddMovementInput` _bp_character (`self.GetActorForwardVector` _bp_character) AxisValue false))

(event `InputAxis|Turn`
  (params (AxisValue :type "Float (single-precision)"))
  ;[1 1 1] Turn
  (`self.AddYawInput` AxisValue))

(event `InputAxis|LookUp`
  (params (AxisValue :type "Float (single-precision)"))
  ;[1 1 1] Turn
  (`self.AddPitchInput` AxisValue))

(event `InputAxis|Right`
  (params (AxisValue :type "Float (single-precision)"))
  (bind _bp_character (`self.BP Character`))
  ;[1 1 1] Move
  (`Pawn.AddMovementInput` _bp_character (`self.GetActorRightVector` _bp_character) AxisValue false))

(fn `UserConstructionScript`)